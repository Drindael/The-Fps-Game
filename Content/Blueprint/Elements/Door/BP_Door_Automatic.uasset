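; Automatic sliding door that moves vertically when something enters its trigger box and returns when it leaves.
; Box overlap begin and end events toggle IsOpen, and each plays its own timeline from the start.
; The timelines offset the Cube's relative Z from InitialCoordonates, with closing counting down from a hardcoded 100-unit raised position.
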(event `self.Box.OnComponentBeginOverlap`
  (params (OverlappedComponent :type "PrimitiveComponent Object Reference") (OtherActor :type "Actor Object Reference") (OtherComp :type "PrimitiveComponent Object Reference") (OtherBodyIndex :type Integer) (bFromSweep :type Boolean) (SweepResult :type "HitResult Structure (by ref)"))
  (bind (_initialcoordonates_x _initialcoordonates_y _initialcoordonates_z) (`KismetMathLibrary.BreakVector` (`self.InitialCoordonates`)))
  ;[1 1 1] Approaching Door
  (if (not (`self.isOpen`))
    (set `self.isOpen` true)
    (bind (_direction _posz) (`Timeline|Timeline` :!via `PlayFromStart`)
      (:`Update`
        (`SceneComponent.K2_SetRelativeLocation` (`self.Cube`) (`KismetMathLibrary.MakeVector` _initialcoordonates_x _initialcoordonates_y (+ _posz _initialcoordonates_z)) false false)))))

(event `self.Box.OnComponentEndOverlap`
  (params (OverlappedComponent :type "PrimitiveComponent Object Reference") (OtherActor :type "Actor Object Reference") (OtherComp :type "PrimitiveComponent Object Reference") (OtherBodyIndex :type Integer))
  (bind (_initialcoordonates_x _initialcoordonates_y _initialcoordonates_z) (`KismetMathLibrary.BreakVector` (`self.InitialCoordonates`)))
  ;[1 1 1] Leaving door
  (if (`self.isOpen`)
    (set `self.isOpen` false)
    (bind (_direction _posz) (`Timeline|Timeline_0` :!via `PlayFromStart`)
      (:`Update`
        (`SceneComponent.K2_SetRelativeLocation` (`self.Cube`) (`KismetMathLibrary.MakeVector` _initialcoordonates_x _initialcoordonates_y (- (+ _initialcoordonates_z 100.0) _posz)) false false)))))

(fn `UserConstructionScript`
  (`parent.UserConstructionScript`))