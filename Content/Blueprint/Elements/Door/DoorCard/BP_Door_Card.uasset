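; BP_Door_Card is a door that opens once red, blue and yellow cards are all inserted.
; Each insert event, gated by that color's active flag, marks the card as in the door, turns off its light, shows its placeholder and plays a sound.
; When all three are in, a Timeline raises or lowers the root component along Z from its relative location.
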(event `InsertRedCard`
  ;[1 0 0] Red Card Interaction
  (if (`self.IsRedActive?`)
    (set `self.IsRedInDoor?` true)
    (`self.SetCard` (`self.RedLight`) (`self.RedCardPlaceholder`))
    (`self.OpenCardDoor`)))

(event `InsertBlueCard`
  ;[0 0.2192 1] Blue Card Interaction
  (if (`self.IsBlueActive?`)
    (set `self.IsBlueInDoor?` true)
    (`self.SetCard` (`self.BlueLight`) (`self.BlueCardPlaceholder`))
    (`self.OpenCardDoor`)))

(event `InsertYellowCard`
  ;[1 0.8936 0] Yellow Card Interaction
  (if (`self.IsYellowActive?`)
    (set `self.IsYellowInDoor?` true)
    (`self.SetCard` (`self.YellowLight`) (`self.YellowCardPlaceholder`))
    (`self.OpenCardDoor`)))

(event `SetCard`
  (params (Light :type "LightComponent Object Reference") (Card :type "SceneComponent Object Reference"))
  ;[1 1 1] Turn off the light and place the card holder
  (`LightComponent.SetIntensity` Light 0.0)
  (`SceneComponent.SetVisibility` Card true false)
  (`GameplayStatics.PlaySound2D` "/Engine/VREditor/Sounds/UI/Camera_Shutter.Camera_Shutter" 1.0 1.0 0.0 null null))

(event `OpenCardDoor`
  (bind _defaultsceneroot (`self.DefaultSceneRoot`))
  ;[1 1 1] Try to open the door
  (if (and (and (`self.IsBlueInDoor?`) (`self.IsRedInDoor?`)) (and (`self.IsYellowInDoor?`) true))
    (`self.OpenDoor` _defaultsceneroot (`SceneComponent.RelativeLocation` _defaultsceneroot))))

(event `OpenDoor`
  (params (Target :type "SceneComponent Object Reference") (VectorPos :type "Vector Structure"))
  ;[1 1 1] Move Door
  (bind (_direction _posz) (`Timeline|Timeline`)
    (:`Update`
      (`SceneComponent.K2_SetRelativeLocation` Target (`KismetMathLibrary.MakeVector` VectorPos_X VectorPos_Y (+ _posz VectorPos_Z)) false false))))

(fn `UserConstructionScript`
  (`parent.UserConstructionScript`))