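; Yellow glass special card actor that, when interacted with, reveals a temporary solid cube.
; The cube starts hidden with collision disabled on BeginPlay.
; Interact shows it, enables query and physics collision, and applies the laser pointer material to the sphere components.
; After a ten-second delay the whole actor destroys itself.
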(event `self.ReceiveBeginPlay`
  (bind _cube (`self.Cube`))
  (`SceneComponent.SetVisibility` _cube false false)
  (`PrimitiveComponent.SetCollisionEnabled` _cube "NoCollision"))

(event `self.Interact`
  (params (`Character Picking Up` :type "/Game/FirstPerson/Blueprints/BP_FirstPersonCharacter Object Reference"))
  (bind _cube (`self.Cube`))
  (`SceneComponent.SetVisibility` _cube true false)
  (`PrimitiveComponent.SetCollisionEnabled` _cube "QueryAndPhysics")
  (`PrimitiveComponent.SetMaterial` (`self.Sphere`) 0 "/Engine/VREditor/LaserPointer/LaserPointerMaterial.LaserPointerMaterial")
  (`PrimitiveComponent.SetMaterial` (`self.Sphere`) 0 "/Engine/VREditor/LaserPointer/LaserPointerMaterial.LaserPointerMaterial")
  (`KismetSystemLibrary.Delay` 10.0)
  (`self.K2_DestroyActor`))

(fn `UserConstructionScript`)