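; BP_GlassCard is a special card actor that, when interacted with, turns on a solid cube and spawns four spawners.
; The cube starts hidden without collision, and Interact makes it visible and collidable and applies a laser pointer material to the sphere.
; SpawnSpawner places a BP_Spawner at each of four marker component locations.
; The card destroys itself 15 seconds after activation.
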(event `self.ReceiveBeginPlay`
  (bind _cube (`self.Cube`))
  (`SceneComponent.SetVisibility` _cube false false)
  (`PrimitiveComponent.SetCollisionEnabled` _cube "NoCollision"))

(event `/Game/Blueprint/Interface/BPI_Interact.Interact`
  (params (`Character Picking Up` :type "/Game/FirstPerson/Blueprints/BP_FirstPersonCharacter Object Reference"))
  (bind _cube (`self.Cube`))
  (`SceneComponent.SetVisibility` _cube true false)
  (`PrimitiveComponent.SetCollisionEnabled` _cube "QueryAndPhysics")
  (`PrimitiveComponent.SetMaterial` (`self.Sphere`) 0 "/Engine/VREditor/LaserPointer/LaserPointerMaterial.LaserPointerMaterial")
  (`PrimitiveComponent.SetMaterial` (`self.Sphere`) 0 "/Engine/VREditor/LaserPointer/LaserPointerMaterial.LaserPointerMaterial")
  (`self.SpawnSpawner` (`self.spawner1pos`))
  (`self.SpawnSpawner` (`self.spawner1pos1`))
  (`self.SpawnSpawner` (`self.spawner1pos2`))
  (`self.SpawnSpawner` (`self.spawner1pos3`))
  (`KismetSystemLibrary.Delay` 15.0)
  (`self.K2_DestroyActor`))

(event `SpawnSpawner`
  (params (Target :type "SceneComponent Object Reference"))
  (`|SpawnActorFromClass` "/Game/Blueprint/Elements/BP_Spawner.BP_Spawner_C" (`KismetMathLibrary.MakeTransform` (`SceneComponent.K2_GetComponentLocation` Target)) "AlwaysSpawn" "MultiplyWithRoot" null null))

(fn `UserConstructionScript`)