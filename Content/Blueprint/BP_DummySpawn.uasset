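; BP_DummySpawn is an actor that opens the main menu and prepares player input when play begins.
; On BeginPlay it adds WBP_MainMenu to the viewport, switches player 0 to UI-only input and shows the mouse cursor.
; It then adds the IMC_Player Enhanced Input mapping context and registers it with the user settings if it is not already registered.
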(event `self.ReceiveBeginPlay`
  (bind _returnvalue (`GameplayStatics.GetPlayerController` 0))
  (bind _returnvalue_2 (pcsubsystem `EnhancedInputLocalPlayerSubsystem` (`GameplayStatics.GetPlayerController` 0)))
  (bind _returnvalue_3 (`EnhancedInputSubsystemInterface.GetUserSettings` _returnvalue_2))
  (bind _returnvalue_4 (`|CreateWidget` "/Game/UI/WBP_MainMenu.WBP_MainMenu_C"))
  (`UserWidget.AddToViewport` _returnvalue_4 0)
  (`WidgetBlueprintLibrary.SetInputMode_UIOnlyEx` _returnvalue _returnvalue_4)
  (set `PlayerController.bShowMouseCursor` true _returnvalue)
  (`/Engine/EditorBlueprintResources/StandardMacros.IsValid` _returnvalue_2
    (:`Is Valid`
      (`EnhancedInputSubsystemInterface.AddMappingContext` _returnvalue_2 "/Game/FirstPerson/Input/IMC_Player.IMC_Player" 0 (struct))
      (if (not (`EnhancedInputUserSettings.IsMappingContextRegistered` _returnvalue_3 "/Game/FirstPerson/Input/IMC_Player.IMC_Player"))
        (`EnhancedInputUserSettings.RegisterInputMappingContext` _returnvalue_3 "/Game/FirstPerson/Input/IMC_Player.IMC_Player")))))

(fn `UserConstructionScript`)