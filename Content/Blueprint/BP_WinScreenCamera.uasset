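; BP_WinScreenCamera is the win screen actor, which brings up the victory menu when play begins.
; On BeginPlay it creates WBP_WinMenu, adds it to the viewport, switches the player to UI-only input focused on that widget, and shows the mouse cursor.
; An unconnected chain that would add and register the IMC_Player Enhanced Input mapping context never runs.
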(event `self.ReceiveBeginPlay`
  (bind _returnvalue (`GameplayStatics.GetPlayerController` 0))
  (bind _returnvalue_2 (`|CreateWidget` "/Game/UI/WBP_WinMenu.WBP_WinMenu_C"))
  (`UserWidget.AddToViewport` _returnvalue_2 0)
  (`WidgetBlueprintLibrary.SetInputMode_UIOnlyEx` _returnvalue _returnvalue_2)
  (set `PlayerController.bShowMouseCursor` true _returnvalue))

(fn `UserConstructionScript`)