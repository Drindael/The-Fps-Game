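; Ranged AI enemy character that runs the BT_Ai_Range behavior tree on the BB_BT_AI blackboard and awards score to the player when killed.
; AI Perception updates toggle the "CanSeePlayer?" key and switch walk speed between chase and patrol.
; Damage reduces health, playing hit feedback or a death sequence that stops movement, detaches the controller and destroys the actor after a delay.
; A separate event plays the shoot montage and sound.
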(event `self.ReceiveAnyDamage`
  (params (Damage :type "Float (single-precision)") (DamageType :type "DamageType Object Reference") (InstigatedBy :type "Controller Object Reference") (DamageCauser :type "Actor Object Reference"))
  (if (not (`self.isDead?`))
    (bind _output_get (set `self.Health` (- (`self.Health`) Damage)))
    (if (<= _output_get 0.0)
      (bind _asbp_first_person_character (cast `/Game/FirstPerson/Blueprints/BP_FirstPersonCharacter` (`GameplayStatics.GetPlayerCharacter` 0)))
      (`/Game/FirstPerson/Blueprints/BP_FirstPersonCharacter.Adding Score` _asbp_first_person_character (`self.score`))
      (`self.PlayDieAnimation`)
      (`self.DetachFromControllerPendingDestroy`)
      (`KismetSystemLibrary.Delay` 3.0)
      (`self.K2_DestroyActor`)
      (else
        (`self.PlayHitAnimation*`)))))

(event `self.ReceiveBeginPlay`
  (bind _returnvalue (`AIBlueprintHelperLibrary.GetAIController` self))
  (`GameplayStatics.PlaySoundAtLocation` "/Game/Blueprint/AI/resources/sfx/range/rangeSpawn.rangeSpawn" (`self.K2_GetActorLocation` self) (struct) 1.0 1.0 0.0 "/Game/Sound/SA_Natural.SA_Natural" null self null)
  (`AIController.UseBlackboard` _returnvalue "/Game/Blueprint/AI/BehaviorTree/BB_BT_AI.BB_BT_AI")
  (`AIController.RunBehaviorTree` _returnvalue "/Game/Blueprint/AI/BehaviorTree/BT_Ai_Range.BT_Ai_Range"))

(event `self.AIPerception.OnTargetPerceptionUpdated`
  (params (Actor :type "Actor Object Reference") (Stimulus :type "AIStimulus Structure"))
  (bind _returnvalue (`AIBlueprintHelperLibrary.GetBlackboard` null))
  (if (`self.isDead?`)
    _
    (elif Stimulus_bSuccessfullySensed
      (`BlackboardComponent.SetValueAsBool` _returnvalue "CanSeePlayer?" true)
      (set `CharacterMovementComponent.MaxWalkSpeed` (`self.ChaseSpeed`) (`self.CharacterMovement`))
      (else
        (`BlackboardComponent.SetValueAsBool` _returnvalue "CanSeePlayer?" false)
        (set `CharacterMovementComponent.MaxWalkSpeed` (`self.PatrolSpeed`) (`self.CharacterMovement`))))))

(event `PlayShootAnimation`
  (`GameplayStatics.PlaySound2D` "/Game/Blueprint/AI/resources/sfx/range/rangeAttack.rangeAttack" 1.0 1.0 0.0 null null)
  (`self.PlayAnimMontage` "/Game/Blueprint/AI/resources/Range/source/animation/sequences/AM_Range_Attack.AM_Range_Attack"))

(event `PlayHitAnimation*`
  (`self.PlayAnimMontage` "/Game/Blueprint/AI/resources/Range/source/animation/sequences/AM_Range_Hit.AM_Range_Hit")
  (`GameplayStatics.PlaySound2D` "/Game/Blueprint/AI/resources/sfx/range/rangeHit.rangeHit" 1.0 1.0 0.0 null null))

(event `PlayDieAnimation`
  (`self.PlayAnimMontage` "/Game/Blueprint/AI/resources/Range/source/animation/sequences/AM_Range_Die.AM_Range_Die")
  (`CharacterMovementComponent.SetMovementMode` (`self.CharacterMovement`) "MOVE_None" 0)
  (`GameplayStatics.PlaySound2D` "/Game/Blueprint/AI/resources/sfx/range/rangeDie.rangeDie" 1.0 1.0 0.0 null null)
  (set `self.isDead?` true))

(fn `UserConstructionScript`
  (set `self.ChaseSpeed` 500.0)
  (set `self.PatrolSpeed` 350.0))