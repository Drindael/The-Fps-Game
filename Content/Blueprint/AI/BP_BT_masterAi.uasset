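; Master AI character that patrols or chases the player and can take damage and die.
; On BeginPlay it runs BT_Ai with BB_BT_AI; perception updates set the CanSeePlayer? key and switch between chase and patrol speeds.
; JumponDestination launches it along a suggested projectile arc while the player is seen.
; Damage reduces health and plays a hit montage, or on death plays a die montage, detaches the controller and destroys the actor after a delay.
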(event `self.ReceiveBeginPlay`
  (bind _returnvalue (`AIBlueprintHelperLibrary.GetAIController` self))
  (`AIController.UseBlackboard` _returnvalue "/Game/Blueprint/AI/BehaviorTree/BB_BT_AI.BB_BT_AI")
  (`AIController.RunBehaviorTree` _returnvalue "/Game/Blueprint/AI/BehaviorTree/BT_Ai.BT_Ai"))

(event `self.AIPerception.OnTargetPerceptionUpdated`
  (params (Actor :type "Actor Object Reference") (Stimulus :type "AIStimulus Structure"))
  (bind _returnvalue (`AIBlueprintHelperLibrary.GetBlackboard` null))
  (if (`self.isDead?`)
    _
    (elif Stimulus_bSuccessfullySensed
      (`BlackboardComponent.SetValueAsBool` _returnvalue "CanSeePlayer?" true)
      (set `CharacterMovementComponent.MaxWalkSpeed` (`self.ChaseSpeed`) (`self.CharacterMovement`))
      (`KismetSystemLibrary.PrintString` "see player" true true (struct :`G` 1.0 :`B` 0.059379 :`A` 1.0))
      (else
        (`BlackboardComponent.SetValueAsBool` _returnvalue "CanSeePlayer?" false)
        (set `CharacterMovementComponent.MaxWalkSpeed` (`self.PatrolSpeed`) (`self.CharacterMovement`))
        (`KismetSystemLibrary.PrintString` "Loose sight" true true (struct :`R` 1.0 :`B` 0.233937 :`A` 1.0))))))

(event `/Game/Blueprint/AI/Interfaces/BPI_MyInterfaces.JumpOnDestination`
  (params (Destination :type "Vector Structure"))
  (if (`BlackboardComponent.GetValueAsBool` (`AIBlueprintHelperLibrary.GetBlackboard` null) "CanSeePlayer?")
    (bind _outlaunchvelocity (`GameplayStatics.SuggestProjectileVelocity_CustomArc` (`self.K2_GetActorLocation`) (`KismetMathLibrary.MakeVector` (.x Destination) (.y Destination) (+ (.z Destination) 250.0))))
    (`self.LaunchCharacter` _outlaunchvelocity true true)))

(event `self.ReceiveAnyDamage`
  (params (Damage :type "Float (single-precision)") (DamageType :type "DamageType Object Reference") (InstigatedBy :type "Controller Object Reference") (DamageCauser :type "Actor Object Reference"))
  (if (not (`self.isDead?`))
    (bind _output_get (set `self.Health` (- (`self.Health`) Damage)))
    (if (<= _output_get 0.0)
      (`self.PlayDieAnimation`)
      (`self.DetachFromControllerPendingDestroy`)
      (`KismetSystemLibrary.Delay` 3.0)
      (`self.K2_DestroyActor`)
      (else
        (`self.PlayHitAnimation*`)))))

(event `PlayHitAnimation*`
  (`self.PlayAnimMontage` (`self.Hit Animation`)))

(event `PlayAttackAnimation`
  (`self.PlayAnimMontage` (`self.AttackAnimation`)))

(event `PlayDieAnimation`
  (`self.PlayAnimMontage` (`self.Die Animation`))
  (`CharacterMovementComponent.SetMovementMode` (`self.CharacterMovement`) "MOVE_None" 0)
  (set `self.isDead?` true))

(fn `UserConstructionScript`)