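; BP_Laser_Trap is a moving hazard that damages the first-person character when its Cylinder component registers a hit.
; The construction script gives InterpToMovement a randomized duration and a relative path from the origin to the Pos variable.
; A hit on the character applies fixed damage, then a boolean gate and short delay act as a cooldown.
; Leftover debug prints remain in the hit logic.
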(event `self.ReceiveBeginPlay`)

(event `self.Cylinder.OnComponentHit`
  (params (HitComponent :type "PrimitiveComponent Object Reference") (OtherActor :type "Actor Object Reference") (OtherComp :type "PrimitiveComponent Object Reference") (NormalImpulse :type "Vector Structure") (Hit :type "HitResult Structure (by ref)"))
  (if (`self.dmgAvalaible`)
    (bind _asbp_first_person_character (cast `/Game/FirstPerson/Blueprints/BP_FirstPersonCharacter` OtherActor)
      (:`then`
        (`GameplayStatics.ApplyDamage` _asbp_first_person_character 15.0)
        (`KismetSystemLibrary.PrintString` "Hello")
        (set `self.dmgAvalaible` false)
        (`KismetSystemLibrary.Delay` 1.0)
        (set `self.dmgAvalaible` true))
      (:`CastFailed`
        (`KismetSystemLibrary.PrintString` "Hello")))))

(fn `UserConstructionScript`
  (bind _interptomovement (`self.InterpToMovement`))
  (set `InterpToMovementComponent.Duration` (`KismetMathLibrary.RandomFloatInRange` 2.0 4.0) _interptomovement)
  (`InterpToMovementComponent.AddControlPointPosition` _interptomovement (0.0 0.0 0.0) true)
  (`InterpToMovementComponent.AddControlPointPosition` _interptomovement (`self.pos`) true))