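; BP_AmmoPickUp is an interactable ammo pickup prop for pistol, shotgun, assault rifle or sniper ammunition.
; On BeginPlay it switches on TypeOfAmmo to set the matching static mesh on PickUpObject.
; When interacted with, it calls AddingAmmo on the interacting character with its ammo amount and type, then destroys itself.
; The mesh is chosen at runtime, as the construction script only calls its parent.
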(event `self.ReceiveBeginPlay`
  (bind _pickupobject (`self.PickUpObject`))
  (`parent.ReceiveBeginPlay`)
  (switch `/Game/Blueprint/Props/Weapon/E_WeaponType` (`self.Type Of Ammo`)
    (:`NewEnumerator1`
      (`StaticMeshComponent.SetStaticMesh` _pickupobject "/Game/MilitaryWeapSilver/Pickups/Pistol_Pickup.Pistol_Pickup"))
    (:`NewEnumerator2`
      (`StaticMeshComponent.SetStaticMesh` _pickupobject "/Game/MilitaryWeapSilver/Pickups/Shotgun_Pickup.Shotgun_Pickup"))
    (:`NewEnumerator3`
      (`StaticMeshComponent.SetStaticMesh` _pickupobject "/Game/MilitaryWeapSilver/Pickups/AssaultRifle_Pickup.AssaultRifle_Pickup"))
    (:`NewEnumerator4`
      (`StaticMeshComponent.SetStaticMesh` _pickupobject "/Game/MilitaryWeapSilver/Pickups/SniperRifle_Pickup.SniperRifle_Pickup"))))

(event `/Game/Blueprint/Interface/BPI_Interact.Interact`
  (params (`Character Picking Up` :type "/Game/FirstPerson/Blueprints/BP_FirstPersonCharacter Object Reference"))
  (`/Game/FirstPerson/Blueprints/BP_FirstPersonCharacter.Adding Ammo` `Character Picking Up` (`self.Ammo`) (`self.Type Of Ammo`))
  (`self.K2_DestroyActor`))

(fn `UserConstructionScript`
  (`parent.UserConstructionScript`))