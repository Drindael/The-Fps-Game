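; Base Blueprint for a ranged AI character that patrols and chases the player.
; On BeginPlay its AI controller loads the BB_BT_AI blackboard and runs the BT_Ai_Range behavior tree.
; AI Perception updates set the "CanSeePlayer?" blackboard key and switch walk speed between chase and patrol values.
; The construction script initializes both speeds.
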(event `self.ReceiveBeginPlay`
  (bind _returnvalue (`AIBlueprintHelperLibrary.GetAIController` self))
  (`AIController.UseBlackboard` _returnvalue "/Game/Blueprints/AI/BehaviorTree/BB_BT_AI.BB_BT_AI")
  (`AIController.RunBehaviorTree` _returnvalue "/Game/Blueprints/AI/BehaviorTree/BT_Ai_Range.BT_Ai_Range"))

(event `self.AIPerception.OnTargetPerceptionUpdated`
  (params (Actor :type "Actor Object Reference") (Stimulus :type "AIStimulus Structure"))
  (bind _returnvalue (`AIBlueprintHelperLibrary.GetBlackboard` null))
  (if Stimulus_bSuccessfullySensed
    (`BlackboardComponent.SetValueAsBool` _returnvalue "CanSeePlayer?" true)
    (set `CharacterMovementComponent.MaxWalkSpeed` (`self.ChaseSpeed`) (`self.CharacterMovement`))
    (else
      (`BlackboardComponent.SetValueAsBool` _returnvalue "CanSeePlayer?" false)
      (set `CharacterMovementComponent.MaxWalkSpeed` (`self.PatrolSpeed`) (`self.CharacterMovement`)))))

(fn `UserConstructionScript`
  (set `self.ChaseSpeed` 500.0)
  (set `self.PatrolSpeed` 350.0))