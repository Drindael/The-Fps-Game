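; Master AI pawn that wanders near the player, chases on perception and destroys itself when health runs out.
; AI Perception toggles CanSeePlayer, switching between chasing the sensed character and moving to random reachable points around the player's location.
; Successful moves from both behaviors share a random delay, then re-check sight to choose the next move.
; Each TakeDamage call decrements health by one.
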(event `self.ReceiveBeginPlay`
  (`self.GoToPatrol`))

(event `self.AIPerception.OnTargetPerceptionUpdated`
  (params (Actor :type "Actor Object Reference") (Stimulus :type "AIStimulus Structure"))
  (if Stimulus_bSuccessfullySensed
    (set `self.CanSeePlayer?` true)
    (bind _asbp_first_person_character (cast `/Game/FirstPerson/Blueprints/BP_FirstPersonCharacter` Actor))
    (`self.GoToPlayer` _asbp_first_person_character)
    (else
      (set `self.CanSeePlayer?` false)
      (`self.GoToPatrol`))))

(event `GoToPlayer`
  (params (TargetActor :type "Actor Object Reference"))
  (`KismetSystemLibrary.PrintString` "GoToPlayer")
  (`|AIMoveTo` self (0.0 0.0 0.0) TargetActor 5.0 true
    (:`OnSuccess`
      (`KismetSystemLibrary.Delay` (`KismetMathLibrary.RandomFloatInRange` 1.5 4.0) :!label _label)
      (if (`self.CanSeePlayer?`)
        (`self.GoToPlayer` TargetActor)
        (else
          (`self.GoToPatrol`))))))

(event `GoToPatrol`
  (`KismetSystemLibrary.PrintString` "GoToPatrol")
  (`|AIMoveTo` self (`NavigationSystemV1.K2_GetRandomReachablePointInRadius` (`self.K2_GetActorLocation` (`GameplayStatics.GetPlayerCharacter` 0)) 500.0 null null) null 100.0 true
    (:`OnSuccess`
      (goto _label))))

(event `TakeDamage`
  (`KismetSystemLibrary.PrintString` "TakeDamage")
  (bind _result (`/Engine/EditorBlueprintResources/StandardMacros.DecrementInt` (`self.CurrentHealth`))
    (:`  `
      (if (<= _result 0)
        (`self.K2_DestroyActor`)))))

(fn `UserConstructionScript`)